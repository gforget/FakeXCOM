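; Gameplay ability under AlienSoldier that heals a selected ally by a percentage of its max health in turn-based tactical combat.
; Target filtering keeps only units below max health, and the ability disables itself with a reason when no actions or targets remain.
; HealingPercent of the target's max health, rounded up, becomes both min and max dynamic value.
; Activation spends one action, heals the TargetManager's selected target, then ends.
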(event `self.SetAbilityEnabledEvent`
  (params (Unit :type "Unit Object Reference"))
  (set `self.OwningUnitRef` Unit)
  (if (== (`Unit.GetActions` (`self.OwningUnitRef`)) 0)
    (set `self.AbilityDisabledText` "No actions left to use this ability")
    (`self.SetIsDisabled` (`self.OwningUnitRef`) true)
    (elif (== (`KismetArrayLibrary.Array_Length` (`.AllAvailableUnitTargets` (break `UnitAbilityInfoStruct` (`BlueprintMapLibrary.Map_Find` (`Unit.UnitAbilityInfos` (`self.OwningUnitRef`)) (`self.AbilityId`))))) 0)
      (set `self.AbilityDisabledText` "No target available to use this ability")
      (`self.SetIsDisabled` (`self.OwningUnitRef`) true)
      (else
        (`self.SetIsDisabled` (`self.OwningUnitRef`))))))

(event `self.SetDynamicDamageValueEvent`
  (params (Unit :type "Unit Object Reference") (Target :type "Actor Object Reference"))
  (bind _returnvalue (`KismetMathLibrary.FCeil` (* (`Unit.GetMaxHealth` (`self.TargetUnitRef`)) (/ (`self.HealingPercent`) 100.0))))
  (set `self.OwningUnitRef` Unit)
  (bind _output_get (set `self.TargetActorRef` Target))
  (bind _asunit (cast `Unit` _output_get))
  (set `self.TargetUnitRef` _asunit)
  (`self.SetDynamicDamageValue` (`self.OwningUnitRef`) (`self.TargetActorRef`) _returnvalue _returnvalue))

(event `self.K2_ActivateAbility`
  (bind _asunit (cast `Unit` (`self.GetOwningActorFromActorInfo`)))
  (set `self.OwningUnitRef` _asunit)
  (set `self.TargetActorRef` (`TargetManager.GetCurrentlySelectedTarget` (`TBTacticalGameMode.TargetManager` (`self.GetTBTacticalGameMode`))))
  (`self.CostActions` (`self.OwningUnitRef`) (`KismetMathLibrary.FTrunc` 1.0))
  (`self.ApplyHeal` (`self.TargetActorRef`) (`self.GetDamageValue` (`self.OwningUnitRef`) (`self.TargetActorRef`)))
  (`self.EndUnitAbility`))

(fn `FilterTargets`
  (params (OwningUnit :type "Unit Object Reference") (TargetActor :type "Actor Object Reference"))
  (returns (ReturnValue :type Boolean))
  (locals (TargetUnitRef :type "Unit Object Reference"))
  (bind _asunit (cast `Unit` TargetActor))
  (set `local.TargetUnitRef` _asunit)
  (return (< (`Unit.GetHealth` (`local.TargetUnitRef`)) (`Unit.GetMaxHealth` (`local.TargetUnitRef`)))))
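; Alien Soldier ability that heals a selected ally in turn-based tactical combat.
; Target setup extends the parent's list, then drops units where two attribute values match, likely those at full health.
; The ability is always visible but disables with a reason when no actions or targets remain.
; Activation spends an action, applies a rounded random heal within the unit's dynamic damage range, then ends the ability.
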(event `self.SetTargets`
  (params (IdUnit :type Integer))
  (bind _output_get (set `self.Id Unit` IdUnit))
  (`parent.SetTargets` _output_get)
  (bind _returnvalue (`UnitManager.GetUnitFromId` (`TBTacticalGameMode.UnitManager` (`self.GetTBTacticalGameMode`)) (`self.Id Unit`)))
  (set `self.Unit` _returnvalue)
  (`KismetArrayLibrary.Array_Clear` (`self.TargetUnitsToRemove`))
  (for _array_element (`.AllAvailableTargets` (break `UnitAbilityInfoStruct` (`BlueprintMapLibrary.Map_Find` (`Unit.UnitAbilityInfos` (`self.Unit`)) (`self.AbilityId`))))
    (bind _asunit (cast `Unit` _array_element))
    (set `self.TargetUnit` _asunit)
    (if (== (`.ReturnValue` (`AbilitySystemComponent.GetGameplayAttributeValue` (`AbilitySystemBlueprintLibrary.GetAbilitySystemComponent` (`self.TargetUnit`)) (struct :`AttributeName` "Health" :`Attribute` "/Script/FakeXCOM.UnitAttributeSet:Health" :`AttributeOwner` "/Script/CoreUObject.Class'/Script/FakeXCOM.UnitAttributeSet'"))) (`.ReturnValue` (`AbilitySystemComponent.GetGameplayAttributeValue` (`AbilitySystemBlueprintLibrary.GetAbilitySystemComponent` (`self.TargetUnit`)) (struct :`AttributeName` "MaxHealth" :`Attribute` "/Script/FakeXCOM.UnitAttributeSet:MaxHealth" :`AttributeOwner` "/Script/CoreUObject.Class'/Script/FakeXCOM.UnitAttributeSet'"))))
      (`KismetArrayLibrary.Array_Add` (`self.TargetUnitsToRemove`) (`Unit.IdUnit` (`self.TargetUnit`)))))
  (`self.RemoveTargets` (`Unit.IdUnit` (`self.Unit`)) (`self.TargetUnitsToRemove`))
  (`self.EndSetTargets` (`Unit.IdUnit` (`self.Unit`))))

(event `self.SetAbilityHiddenEvent`
  (params (Unit :type "Unit Object Reference"))
  (set `self.Unit` Unit)
  (`self.SetIsHidden` (`self.Unit`)))

(event `self.SetAbilityEnabledEvent`
  (params (Unit :type "Unit Object Reference"))
  (set `self.Unit` Unit)
  (if (== (`.ReturnValue` (`AbilitySystemComponent.GetGameplayAttributeValue` (`AbilitySystemBlueprintLibrary.GetAbilitySystemComponent` (`self.Unit`)) (struct :`AttributeName` "Actions" :`Attribute` "/Script/FakeXCOM.UnitAttributeSet:Actions" :`AttributeOwner` "/Script/CoreUObject.Class'/Script/FakeXCOM.UnitAttributeSet'"))) 0.0)
    (set `self.AbilityDisabledText` "No Actions left to use this ability")
    (`self.SetIsDisabled` (`self.Unit`) true)
    (elif (== (`KismetArrayLibrary.Array_Length` (`.AllAvailableTargets` (break `UnitAbilityInfoStruct` (`BlueprintMapLibrary.Map_Find` (`Unit.UnitAbilityInfos` (`self.Unit`)) (`self.AbilityId`))))) 0)
      (set `self.AbilityDisabledText` "No Targets available to use this ability")
      (`self.SetIsDisabled` (`self.Unit`) true)
      (else
        (`self.SetIsDisabled` (`self.Unit`))))))

(event `self.K2_ActivateAbility`
  (bind _idunit (`Unit.IdUnit` (`self.Unit`)))
  (bind _asunit (cast `Unit` (`self.GetOwningActorFromActorInfo`)))
  (set `self.Unit` _asunit)
  (`self.CostActions` (`Unit.IdUnit` (`self.Unit`)) 1.0)
  (`self.ApplyHeal` (`TargetManager.GetCurrentlySelectedTarget` (`TBTacticalGameMode.TargetManager` (`self.GetTBTacticalGameMode`))) (`KismetMathLibrary.Conv_IntToDouble` (`KismetMathLibrary.Round` (`KismetMathLibrary.RandomFloatInRange` (`self.GetDynamicMinDamageValue` _idunit) (`self.GetDynamicMaxDamageValue` _idunit)))))
  (`UnitManager.EndOfAbility` (`TBTacticalGameMode.UnitManager` (`self.GetTBTacticalGameMode`)))
  (`self.K2_EndAbility`))
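; Self-heal ability for the Alien Soldier that lets a unit restore its own health.
; It is hidden while the unit is at full health and disabled with an explanatory message when no actions remain.
; On activation it spends one action, applies a non-critical heal to the owning unit using the ability's damage value as the amount, then ends the ability.
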(event `self.SetAbilityHiddenEvent`
  (params (Unit :type "Unit Object Reference"))
  (set `self.OwningUnitRef` Unit)
  (`self.SetIsHidden` (`self.OwningUnitRef`) (== (`Unit.GetHealth` (`self.OwningUnitRef`)) (`Unit.GetMaxHealth` (`self.OwningUnitRef`)))))

(event `self.SetAbilityEnabledEvent`
  (params (Unit :type "Unit Object Reference"))
  (set `self.OwningUnitRef` Unit)
  (if (== (`Unit.GetActions` (`self.OwningUnitRef`)) 0)
    (set `self.AbilityDisabledText` "No actions left to use this ability")
    (`self.SetIsDisabled` (`self.OwningUnitRef`) true)
    (else
      (`self.SetIsDisabled` (`self.OwningUnitRef`)))))

(event `self.K2_ActivateAbility`
  (bind _owningunitref (`self.OwningUnitRef`))
  (bind _asunit (cast `Unit` (`self.GetOwningActorFromActorInfo`)))
  (set `self.OwningUnitRef` _asunit)
  (`self.CostActions` (`self.OwningUnitRef`) (`KismetMathLibrary.FTrunc` 1.0))
  (`self.ApplyHeal` (`self.OwningUnitRef`) (`self.GetDamageValue` _owningunitref _owningunitref))
  (`self.EndUnitAbility`))
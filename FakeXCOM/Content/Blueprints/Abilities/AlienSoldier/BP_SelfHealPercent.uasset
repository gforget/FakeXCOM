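; Alien soldier self-heal ability for a turn-based tactical game, restoring an amount equal to half of one of the unit's attributes, rounded up.
; Hooks set the dynamic min and max to that amount, hide the ability when two attribute values match, and disable it when an attribute, presented as remaining actions, is zero.
; Activation costs one action, applies the rounded heal without crit, then notifies the UnitManager and ends.
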(event `self.SetAbilityHiddenEvent`
  (params (Unit :type "Unit Object Reference"))
  (set `self.UnitRef` Unit)
  (`self.SetIsHidden` (`self.UnitRef`) (== (`.ReturnValue` (`AbilitySystemComponent.GetGameplayAttributeValue` (`AbilitySystemBlueprintLibrary.GetAbilitySystemComponent` (`self.UnitRef`)) (struct :`AttributeName` "Health" :`Attribute` "/Script/FakeXCOM.UnitAttributeSet:Health" :`AttributeOwner` "/Script/CoreUObject.Class'/Script/FakeXCOM.UnitAttributeSet'"))) (`.ReturnValue` (`AbilitySystemComponent.GetGameplayAttributeValue` (`AbilitySystemBlueprintLibrary.GetAbilitySystemComponent` (`self.UnitRef`)) (struct :`AttributeName` "MaxHealth" :`Attribute` "/Script/FakeXCOM.UnitAttributeSet:MaxHealth" :`AttributeOwner` "/Script/CoreUObject.Class'/Script/FakeXCOM.UnitAttributeSet'"))))))

(event `self.SetAbilityEnabledEvent`
  (params (Unit :type "Unit Object Reference"))
  (set `self.UnitRef` Unit)
  (if (== (`.ReturnValue` (`AbilitySystemComponent.GetGameplayAttributeValue` (`AbilitySystemBlueprintLibrary.GetAbilitySystemComponent` (`self.UnitRef`)) (struct :`AttributeName` "Actions" :`Attribute` "/Script/FakeXCOM.UnitAttributeSet:Actions" :`AttributeOwner` "/Script/CoreUObject.Class'/Script/FakeXCOM.UnitAttributeSet'"))) 0.0)
    (set `self.AbilityDisabledText` "No Actions left to use this ability")
    (`self.SetIsDisabled` (`self.UnitRef`) true)
    (else
      (`self.SetIsDisabled` (`self.UnitRef`)))))

(event `self.SetDynamicDamageValueEvent`
  (params (Unit :type "Unit Object Reference") (Target :type "Actor Object Reference"))
  (bind _returnvalue (`KismetMathLibrary.FCeil` (* (`.ReturnValue` (`AbilitySystemComponent.GetGameplayAttributeValue` (`AbilitySystemBlueprintLibrary.GetAbilitySystemComponent` (`self.UnitRef`)) (struct :`AttributeName` "MaxHealth" :`Attribute` "/Script/FakeXCOM.UnitAttributeSet:MaxHealth" :`AttributeOwner` "/Script/CoreUObject.Class'/Script/FakeXCOM.UnitAttributeSet'"))) 0.5)))
  (bind _output_get (set `self.UnitRef` Unit))
  (`self.SetDynamicDamageValue` _output_get _output_get (`KismetMathLibrary.Conv_IntToDouble` _returnvalue) (`KismetMathLibrary.Conv_IntToDouble` _returnvalue)))

(event `self.K2_ActivateAbility`
  (bind _unitref (`self.UnitRef`))
  (bind _asunit (cast `Unit` (`self.GetOwningActorFromActorInfo`)))
  (set `self.UnitRef` _asunit)
  (`self.CostActions` (`self.UnitRef`) 1.0)
  (`self.ApplyHeal` (`self.UnitRef`) (`KismetMathLibrary.Conv_IntToDouble` (`KismetMathLibrary.Round` (`KismetMathLibrary.RandomFloatInRange` (`self.GetDynamicMinDamageValue` _unitref _unitref) (`self.GetDynamicMaxDamageValue` _unitref _unitref)))))
  (`UnitManager.EndOfAbility` (`TBTacticalGameMode.UnitManager` (`self.GetTBTacticalGameMode`)))
  (`self.K2_EndAbility`))
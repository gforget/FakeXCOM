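; BP_HunkerDownAbility is a Hunker Down unit ability that is currently a placeholder with no gameplay effect.
; Its hidden event always hides it for the given unit, and its enabled event disables it with an explanatory message when that unit has zero actions left.
; Activation only prints a debug string and ends the unit ability.
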(event `self.SetAbilityHiddenEvent`
  (params (Unit :type "Unit Object Reference"))
  (`self.SetIsHidden` Unit true))

(event `self.SetAbilityEnabledEvent`
  (params (Unit :type "Unit Object Reference"))
  (set `self.Unit` Unit)
  (if (== (`Unit.GetActions` (`self.Unit`)) 0)
    (set `self.AbilityDisabledText` "No Actions left to use this ability")
    (`self.SetIsDisabled` (`self.Unit`) true)
    (else
      (`self.SetIsDisabled` (`self.Unit`)))))

(event `self.K2_ActivateAbility`
  (`KismetSystemLibrary.PrintString` "HunkerDown")
  (`self.EndUnitAbility`))
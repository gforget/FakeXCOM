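; Reload ability for tactical units that refills the gun's ammo at the cost of one action.
; It is disabled with an explanatory message when the unit has no actions left, and hidden when the gun is already at full ammo.
; On activation it shows a RELOADING alert through the tactical game mode's level UI, spends the action, recharges all ammo and ends the ability.
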(event `self.SetAbilityEnabledEvent`
  (params (Unit :type "Unit Object Reference"))
  (set `self.Unit` Unit)
  (if (== (`Unit.GetActions` (`self.Unit`)) 0)
    (set `self.AbilityDisabledText` "No Actions left to use this ability")
    (`self.SetIsDisabled` (`self.Unit`) true)
    (else
      (`self.SetIsDisabled` (`self.Unit`)))))

(event `self.SetAbilityHiddenEvent`
  (params (Unit :type "Unit Object Reference"))
  (set `self.Unit` Unit)
  (if (== (`Gun.GetAmmo` (`Unit.Gun` (`self.Unit`))) (`Gun.GetMaxAmmo` (`Unit.Gun` (`self.Unit`))))
    (`self.SetIsHidden` (`self.Unit`) true)
    (else
      (`self.SetIsHidden` (`self.Unit`)))))

(event `self.K2_ActivateAbility`
  (bind _asunit (cast `Unit` (`self.GetOwningActorFromActorInfo`)))
  (set `self.Unit` _asunit)
  (`LevelUI.BPCallCustomAlertStatusEvent` (`TBTacticalGameMode.LevelUIRef` (`self.GetTBTacticalGameMode`)) (`self.Unit`) (make `Color` 0 255 0 255) "RELOADING" -1.0)
  (`self.CostActions` (`self.Unit`) (`KismetMathLibrary.FTrunc` 1.0))
  (`self.RechargeAllAmmo` (`Unit.Gun` (`self.Unit`)))
  (`self.EndUnitAbility`))
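; Gameplay ability for a tactical unit's gun shot at the selected target, spending all actions and one ammo.
; Setter events feed range, damage, hit and crit values from the gun, and disable the ability without targets, actions or ammo.
; Hit chance combines a range curve, aim, defence, cover and height advantage; cover negates crits.
; Activation locks the camera behind the shooter, rolls hit and crit for damage or a miss, then restores the view.
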(event `self.SetDynamicRangeValueEvent`
  (params (Unit :type "Unit Object Reference"))
  (`self.SetDynamicRangeValue` Unit (`Gun.GetRange` (`Unit.Gun` Unit))))

(event `self.SetDynamicDamageValueEvent`
  (params (Unit :type "Unit Object Reference") (Target :type "Actor Object Reference"))
  (bind _gun (`Unit.Gun` Unit))
  (`self.SetDynamicDamageValue` Unit Target (`Gun.GetMinDamage` _gun) (`Gun.GetMaxDamage` _gun)))

(event `self.SetHitChanceEvent`
  (params (Unit :type "Unit Object Reference") (Target :type "Actor Object Reference"))
  (set `self.Unit` Unit)
  (bind _output_get (set `self.Target` Target))
  (bind _asunit (cast `Unit` _output_get))
  (set `self.TargetUnit` _asunit)
  (bind _returnvalue (`self.GetHitChance` (`self.Unit`) (`self.Target`) (`TileMovementComponent.LocatedNodePath` (`Unit.TileMovementComponent` (`self.Unit`))) (`TileMovementComponent.LocatedNodePath` (`Unit.TileMovementComponent` (`self.TargetUnit`)))))
  (set `self.CalculatedHitChance` _returnvalue)
  (`self.SetHitChance` (`self.Unit`) (`self.Target`) (`self.CalculatedHitChance`)))

(event `self.SetCritChanceEvent`
  (params (Unit :type "Unit Object Reference") (Target :type "Actor Object Reference"))
  (set `self.Unit` Unit)
  (bind _output_get (set `self.Target` Target))
  (bind _asunit (cast `Unit` _output_get))
  (set `self.TargetUnit` _asunit)
  (bind _returnvalue (`self.GetCritChance` (`self.Unit`) (`self.Target`) (`TileMovementComponent.LocatedNodePath` (`Unit.TileMovementComponent` (`self.Unit`))) (`TileMovementComponent.LocatedNodePath` (`Unit.TileMovementComponent` (`self.TargetUnit`)))))
  (set `self.CalculatedCritChance` _returnvalue)
  (`self.SetCritChance` (`self.Unit`) (`self.Target`) (`self.CalculatedCritChance`)))

(event `self.SetAbilityEnabledEvent`
  (params (Unit :type "Unit Object Reference"))
  (set `self.Unit` Unit)
  (if (== (`KismetArrayLibrary.Array_Length` (`.AllAvailableUnitTargets` (break `UnitAbilityInfoStruct` (`BlueprintMapLibrary.Map_Find` (`Unit.UnitAbilityInfos` (`self.Unit`)) (`self.AbilityId`))))) 0)
    (set `self.AbilityDisabledText` "No Targets available to use this ability")
    (`self.SetIsDisabled` (`self.Unit`) true)
    (elif (== (`Unit.GetActions` (`self.Unit`)) 0)
      (set `self.AbilityDisabledText` "No Actions left to use this ability")
      (`self.SetIsDisabled` (`self.Unit`) true)
      (elif (== (`Gun.GetAmmo` (`Unit.Gun` (`self.Unit`))) 0)
        (set `self.AbilityDisabledText` "No Ammo left to use this ability")
        (`self.SetIsDisabled` (`self.Unit`) true)
        (else
          (`self.SetIsDisabled` (`self.Unit`)))))))

(event `self.K2_ActivateAbility`
  (bind _unit (`self.Unit`))
  (bind (_returnvalue_roll _returnvalue_pitch _returnvalue_yaw) (`KismetMathLibrary.BreakRotator` (`Actor.K2_GetActorRotation` (`self.Unit`))))
  (bind (_returnvalue_roll_2 _returnvalue_pitch_2 _returnvalue_yaw_2) (`KismetMathLibrary.BreakRotator` (`Actor.K2_GetActorRotation` (`TBTacticalGameMode.MainController` (`self.GetTBTacticalGameMode`)))))
  (bind _asunit (cast `Unit` (`self.GetOwningActorFromActorInfo`)))
  (set `self.Unit` _asunit)
  (`self.CostAllActions` (`self.Unit`))
  (`self.CostAmmo` (`Unit.Gun` (`self.Unit`)) 1)
  (bind _output_get (set `self.Target` (`TargetManager.GetCurrentlySelectedTarget` (`TBTacticalGameMode.TargetManager` (`self.GetTBTacticalGameMode`)))))
  (bind _asunit_2 (cast `Unit` _output_get)
    (:`then`
      (set `self.TargetUnit` _asunit_2)
      (`self.RotateTowardTarget` (`self.Unit`) (`self.TargetUnit`))
      (set `self.OldYaw` _returnvalue_yaw_2)
      (set `self.OldHeight` (`TBTacticalMainController.CurrentHeightCameraValueIndex` (`TBTacticalGameMode.MainController` (`self.GetTBTacticalGameMode`))))
      (`LevelUI.SetControlInterfaceVisibility` (`TBTacticalGameMode.LevelUIRef` (`self.GetTBTacticalGameMode`)) false)
      ;[1 1 1] Move Camera Back
      (`TBTacticalMainController.RotateCameraToSpecificYaw` (`TBTacticalGameMode.MainController` (`self.GetTBTacticalGameMode`)) _returnvalue_yaw)
      (`TBTacticalMainController.GoToActor` (`TBTacticalGameMode.MainController` (`self.GetTBTacticalGameMode`)) (`self.Unit`))
      (`TBTacticalMainController.MoveCameraHeight` (`TBTacticalGameMode.MainController` (`self.GetTBTacticalGameMode`)) 2)
      (`TBTacticalMainController.ForceCameraLock` (`TBTacticalGameMode.MainController` (`self.GetTBTacticalGameMode`)) true)
      (`AbilityTask_WaitDelay.WaitDelay` 1.5
        (:`OnFinish`
          (`self.TryShootUnitTarget` _unit)
          (`LevelUI.BPCallCustomAlertStatusEvent` (`TBTacticalGameMode.LevelUIRef` (`self.GetTBTacticalGameMode`)) _unit (make `Color` 0 165 255 255) "SHOOTING" -1.0)
          (`AbilityTask_WaitDelay.WaitDelay` 1.5
            (:`OnFinish`
              (`TBTacticalMainController.RotateCameraToSpecificYaw` (`TBTacticalGameMode.MainController` (`self.GetTBTacticalGameMode`)) (`self.OldYaw`))
              (`TBTacticalMainController.MoveCameraHeight` (`TBTacticalGameMode.MainController` (`self.GetTBTacticalGameMode`)) (`self.OldHeight`))
              (`TBTacticalMainController.ForceCameraLock` (`TBTacticalGameMode.MainController` (`self.GetTBTacticalGameMode`)) false)
              (`LevelUI.SetControlInterfaceVisibility` (`TBTacticalGameMode.LevelUIRef` (`self.GetTBTacticalGameMode`)) true)
              (`self.EndUnitAbility`))))))
    (:`CastFailed`
      (`UnitManager.EndOfAbility` (`TBTacticalGameMode.UnitManager` (`self.GetTBTacticalGameMode`)))
      (`self.K2_EndAbility`))))

(fn `GetCritChance`
  (params (Unit :type "Unit Object Reference") (Target :type "Actor Object Reference") (UnitNodePath :type "NodePath Object Reference") (TargetNodePath :type "NodePath Object Reference"))
  (returns (ReturnValue :type "Float (single-precision)"))
  (locals (UnitRef :type "Unit Object Reference") (TargetUnitRef :type "Unit Object Reference") (TargetRef :type "Actor Object Reference") (TargetIsUnit :type Boolean) (ReturnedCalculatedCritChance :type "Float (double-precision)"))
  (set `local.UnitRef` Unit)
  (bind _output_get (set `local.TargetRef` Target))
  (bind _asunit (cast `Unit` _output_get)
    (:`then`
      (set `local.TargetIsUnit` true)
      (set `local.TargetUnitRef` _asunit))
    (:`CastFailed`
      (set `local.TargetIsUnit` false)))
  (if (`local.TargetIsUnit`)
    (if (> (`Unit.GetTargetCoverDefenceBonus` (`local.UnitRef`) (`local.TargetUnitRef`) (`TileMovementComponent.LocatedNodePath` (`Unit.TileMovementComponent` (`local.UnitRef`))) (`TileMovementComponent.LocatedNodePath` (`Unit.TileMovementComponent` (`local.TargetUnitRef`)))) 0.0)
      (set `local.ReturnedCalculatedCritChance` 0.0)
      (else
        (set `local.ReturnedCalculatedCritChance` (`Gun.GetCritChance` (`Unit.Gun` (`local.UnitRef`))))))
    (return (`local.ReturnedCalculatedCritChance`))))

(fn `GetHitChance`
  (params (Unit :type "Unit Object Reference") (Target :type "Actor Object Reference") (UnitNodePath :type "NodePath Object Reference") (TargetNodePath :type "NodePath Object Reference"))
  (returns (ReturnValue :type "Float (single-precision)"))
  (locals (TargetUnitRef :type "Unit Object Reference") (UnitRef :type "Unit Object Reference") (TargetRef :type "Actor Object Reference") (TargetNodePathRef :type "NodePath Object Reference") (TargetIsUnit :type Boolean) (ReturnedCalculatedHitChance :type "Float (double-precision)") (UnitNodePathRef :type "NodePath Object Reference"))
  (set `local.UnitRef` Unit)
  (set `local.TargetNodePathRef` TargetNodePath)
  (set `local.UnitNodePathRef` UnitNodePath)
  (bind _output_get (set `local.TargetRef` Target))
  (bind _asunit (cast `Unit` _output_get)
    (:`then`
      (set `local.TargetIsUnit` true)
      (set `local.TargetUnitRef` _asunit))
    (:`CastFailed`
      (set `local.TargetIsUnit` false)))
  (if (`local.TargetIsUnit`)
    (set `local.ReturnedCalculatedHitChance` (`KismetMathLibrary.FClamp` (+ (`self.GetRangeHitChance` (`local.UnitRef`) (`local.TargetRef`) (`local.UnitNodePathRef`) (`local.TargetNodePathRef`)) (`Unit.GetAim` (`local.UnitRef`)) (* (`Unit.GetDefence` (`local.TargetUnitRef`)) -1.0) (* (`Unit.GetTargetCoverDefenceBonus` (`local.UnitRef`) (`local.TargetUnitRef`) (`local.UnitNodePathRef`) (`local.TargetNodePathRef`)) -1.0) (`Unit.GetHeightAdvantageBonus` (`local.UnitRef`) (`local.TargetUnitRef`))) 0.0 100.0))
    (else
      (set `local.ReturnedCalculatedHitChance` 100.0)))
  (return (`local.ReturnedCalculatedHitChance`)))

(fn `GetRangeHitChance`
  (params (Unit :type "Unit Object Reference") (Target :type "Actor Object Reference") (UnitNodePath :type "NodePath Object Reference") (TargetNodePath :type "NodePath Object Reference"))
  (returns (RangeHitChance :type "Float (double-precision)"))
  (return (* (`MyFunctionLibrary.GetRuntimeFloatCurveValue` (`Gun.GetRangeAimValueCurve` (`Unit.Gun` Unit)) (`KismetMathLibrary.SafeDivide` (`self.GetRangeToTarget` Unit Target UnitNodePath TargetNodePath) (`Gun.GetRange` (`Unit.Gun` Unit)))) 100.0)))

(fn `TryShootUnitTarget`
  (params (UnitTarget :type "Unit Object Reference"))
  (if (`self.RollDiceForHit` UnitTarget (`self.Target`))
    (if (`self.RollDiceForCrit` (`self.Unit`) (`self.Target`))
      (set `self.CritMultiplier` (`Gun.GetCritMultiplier` (`Unit.Gun` (`self.Unit`))))
      (set `self.IsCrit` true)
      (else
        (set `self.CritMultiplier` 1.0)
        (set `self.IsCrit` false)))
    (`self.ApplyDamage` (`self.Target`) (* (`self.GetDamageValue` (`self.Unit`) (`TargetManager.GetCurrentlySelectedTarget` (`TBTacticalGameMode.TargetManager` (`self.GetTBTacticalGameMode`)))) (`self.CritMultiplier`)) (`self.IsCrit`))
    (else
      (bind _asunit (cast `Unit` (`self.Target`)))
      (`LevelUI.BPCallStatusEvent` (`TBTacticalGameMode.LevelUIRef` (`self.GetTBTacticalGameMode`)) _asunit "Miss" -1.0))))
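; AI consideration that scores a unit on whether enemies can target it without its cover giving any defence.
; With cover at its node, it scans enemy units whose default ability lists it as an available target, flagging it flanked at the first zero cover bonus.
; It returns MaxScore when that flag equals HaveEffectiveCover, otherwise MinScore, so true rewards being flanked despite the name.
; Without cover it sets MinScore, skipping the scan.
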(fn `ScoreConsideration`
  (params (OwningUnit :type "Unit Object Reference") (TBTacticalGameMode :type "TBTacticalGameMode Object Reference"))
  (returns (ReturnValue :type "Float (single-precision)"))
  (locals (TBTacticalGameModeRef :type "TBTacticalGameMode Object Reference") (OwningUnitRef :type "Unit Object Reference") (OtherUnitRef :type "Unit Object Reference") (NormalizedScore :type "Float (double-precision)") (CoverDefenceScore :type "Float (double-precision)") (OtherDefaultAbilityRef :type "UnitAbility Object Reference") (OtherRangeRef :type "Float (double-precision)") (IsFlanked :type Boolean))
  (set `local.OwningUnitRef` OwningUnit)
  (set `local.TBTacticalGameModeRef` TBTacticalGameMode)
  (set `local.IsFlanked` false)
  (if (> (`KismetArrayLibrary.Array_Length` (`NodePath.AllCoverInfos` (`TileMovementComponent.LocatedNodePath` (`Unit.TileMovementComponent` (`local.OwningUnitRef`))))) 0)
    (bind _values (`BlueprintMapLibrary.Map_Values` (`UnitManager.AllUnitReference` (`TBTacticalGameMode.UnitManager` (`local.TBTacticalGameModeRef`)))))
    (for _array_element _values
      (set `local.OtherUnitRef` _array_element)
      (bind _returnvalue (`FactionManager.GetFactionRelation` (`TBTacticalGameMode.FactionManagerComponent` (`local.TBTacticalGameModeRef`)) (`Unit.Faction` (`local.OtherUnitRef`)) (`Unit.Faction` (`local.OwningUnitRef`))))
      (if (== _returnvalue (`KismetMathLibrary.Conv_ByteToInt` (enumliteral `EFactionRelation` "Enemy")))
        (set `local.OtherDefaultAbilityRef` (`|GetArrayItem` (`Unit.OwnedAbilities` (`local.OtherUnitRef`)) (`|GetArrayItem` (`Unit.DefaultAbilitiesIndexes` (`local.OtherUnitRef`)))))
        (if (!= (`KismetArrayLibrary.Array_Find` (`.AllAvailableTargets` (break `UnitAbilityInfoStruct` (`BlueprintMapLibrary.Map_Find` (`UnitAbility.UnitAbilityInfos` (`local.OtherDefaultAbilityRef`)) (`Unit.IdUnit` (`local.OtherUnitRef`))))) (`local.OwningUnit`)) -1)
          (set `local.CoverDefenceScore` (`Unit.GetTargetCoverDefenceBonus` (`local.OtherUnitRef`) (`local.OwningUnitRef`)))
          (if (== (`local.CoverDefenceScore`) 0.0)
            (set `local.IsFlanked` true)
            (break)))))
    (if (== (`local.IsFlanked`) (`self.HaveEffectiveCover`))
      (set `local.NormalizedScore` (`self.MaxScore`))
      (else
        (set `local.NormalizedScore` (`self.MinScore`))))
    (return (`local.NormalizedScore`))
    (else
      (set `local.NormalizedScore` (`self.MinScore`)))))
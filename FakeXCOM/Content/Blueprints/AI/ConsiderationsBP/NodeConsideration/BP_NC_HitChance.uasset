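; BP_NC_HitChance is an AI node consideration that scores a candidate grid node by the best hit chance a unit would have from it.
; It takes the unit's first default ability and queries that ability's hit chance against every enemy in sight from the target node.
; The highest chance found is multiplied by MaxScore and returned as the node's score.
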(fn `ScoreConsiderationNode`
  (params (OwningUnit :type "Unit Object Reference") (TBTacticalGameMode :type "TBTacticalGameMode Object Reference") (TargetNode :type "NodePath Object Reference"))
  (returns (ReturnValue :type "Float (single-precision)"))
  (locals (OwningUnitRef :type "Unit Object Reference") (TBTacticalGameModeRef :type "TBTacticalGameMode Object Reference") (TargetNodeRef :type "NodePath Object Reference") (DefaultAbilityRef :type "UnitAbility Object Reference") (HighestChance :type "Float (double-precision)") (CurentHitChance :type "Float (single-precision)" :default 0.0))
  (set `local.OwningUnitRef` OwningUnit)
  (set `local.TBTacticalGameModeRef` TBTacticalGameMode)
  (set `local.TargetNodeRef` TargetNode)
  (set `local.DefaultAbilityRef` (`|GetArrayItem` (`Unit.OwnedAbilities` (`local.OwningUnitRef`)) (`|GetArrayItem` (`Unit.DefaultAbilitiesIndexes` (`local.OwningUnitRef`)))))
  (bind _returnvalue (`self.GetAllEnemyUnitInSight` (`local.OwningUnitRef`) (`local.TBTacticalGameModeRef`) (`local.TargetNodeRef`)))
  (for _array_element _returnvalue
    (bind _returnvalue_2 (`UnitAbility.GetHitChance` (`local.DefaultAbilityRef`) (`local.OwningUnitRef`) _array_element (`local.TargetNodeRef`)))
    (set `local.CurentHitChance` _returnvalue_2)
    (if (> (`local.CurentHitChance`) (`local.HighestChance`))
      (set `local.HighestChance` (`local.CurentHitChance`))))
  (return (* (`local.HighestChance`) (`self.MaxScore`))))
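; AI node consideration for the turn-based tactical game that scores a target node by whether the unit can reach it within a number of actions.
; The action budget is MaxNbOfActionsRequire, replaced by the unit's remaining actions when UseRemainingActions is set or fewer remain, overwriting the variable itself.
; It returns TrueScore if the node's step count fits within move distance per action times that budget, otherwise FalseScore.
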(fn `ScoreConsiderationNode`
  (params (OwningUnit :type "Unit Object Reference") (ActionIndex :type Integer) (TBTacticalGameMode :type "TBTacticalGameMode Object Reference") (TargetNode :type "NodePath Object Reference"))
  (returns (ReturnValue :type "Float (single-precision)"))
  (locals (UnitRef :type "Unit Object Reference") (NodeRef :type "NodePath Object Reference") (NormalizedScore :type "Float (double-precision)") (RemainingNBofActions :type Integer))
  (set `local.UnitRef` OwningUnit)
  (set `local.NodeRef` TargetNode)
  (set `local.RemainingNBofActions` (`Unit.GetActions` (`local.UnitRef`)))
  (if (or (`self.UseRemainingActions`) (< (`local.RemainingNBofActions`) (`self.MaxNbOfActionsRequire`)))
    (set `self.MaxNbOfActionsRequire` (`local.RemainingNBofActions`)))
  (if (<= (`NodePath.NbSteps` (`local.NodeRef`)) (* (`Unit.GetMaxMoveDistancePerAction` (`local.UnitRef`)) (`self.MaxNbOfActionsRequire`)))
    (set `local.NormalizedScore` (`self.TrueScore`))
    (else
      (set `local.NormalizedScore` (`self.FalseScore`))))
  (return (`local.NormalizedScore`)))
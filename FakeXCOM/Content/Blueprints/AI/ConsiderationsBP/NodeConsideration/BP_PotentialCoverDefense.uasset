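; AI node consideration that scores a target node by the potential cover defense it offers a unit in tactical, likely turn-based, combat.
; It gets the lowest potential defense for the owning unit at that node through GetLowestPotentialDefence.
; That value is divided by the unit's full-cover defense bonus and multiplied by MaxScore, so the worst-case cover sets the score.
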(fn `ScoreConsiderationNode`
  (params (OwningUnit :type "Unit Object Reference") (TBTacticalGameMode :type "TBTacticalGameMode Object Reference") (TargetNode :type "NodePath Object Reference"))
  (returns (ReturnValue :type "Float (single-precision)"))
  (locals (OwningUnitRef :type "Unit Object Reference") (TBTacticalGameModeRef :type "TBTacticalGameMode Object Reference") (TargetNodeRef :type "NodePath Object Reference"))
  (set `local.OwningUnitRef` OwningUnit)
  (set `local.TBTacticalGameModeRef` TBTacticalGameMode)
  (set `local.TargetNodeRef` TargetNode)
  (bind _returnvalue (`self.GetLowestPotentialDefence` (`local.OwningUnitRef`) (`local.TBTacticalGameModeRef`) (`local.TargetNodeRef`)))
  (return (* (/ _returnvalue (`Unit.FullCoverDefenceBonus` (`local.OwningUnitRef`))) (`self.MaxScore`))))
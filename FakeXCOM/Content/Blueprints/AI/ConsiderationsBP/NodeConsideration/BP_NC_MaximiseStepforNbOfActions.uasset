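; AI node consideration that scores a target tile higher the more of the unit's movement budget it uses.
; The budget is max move distance per action times either the unit's remaining actions or a required action cap, whichever the flag or shortfall selects.
; Nodes within budget score linearly by step count up to the maximum score, floored at the minimum; nodes beyond it get the minimum.
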(fn `ScoreConsiderationNode`
  (params (OwningUnit :type "Unit Object Reference") (ActionIndex :type Integer) (TBTacticalGameMode :type "TBTacticalGameMode Object Reference") (TargetNode :type "NodePath Object Reference"))
  (returns (ReturnValue :type "Float (single-precision)"))
  (locals (UnitRef :type "Unit Object Reference") (NodeRef :type "NodePath Object Reference") (NormalizedScore :type "Float (double-precision)") (CurrentStepsNb :type Integer) (MaxSteps :type Integer) (RemainingNBofActions :type Integer))
  (set `local.UnitRef` OwningUnit)
  (bind _output_get (set `local.NodeRef` TargetNode))
  (set `local.CurrentStepsNb` (`NodePath.NbSteps` _output_get))
  (set `local.RemainingNBofActions` (`Unit.GetActions` (`local.UnitRef`)))
  (if (or (`self.UseRemainingActions`) (< (`local.RemainingNBofActions`) (`self.MaxNbOfActionsRequire`)))
    (set `local.MaxSteps` (* (`local.RemainingNBofActions`) (`Unit.GetMaxMoveDistancePerAction` (`local.UnitRef`))))
    (else
      (set `local.MaxSteps` (* (`Unit.GetMaxMoveDistancePerAction` (`local.UnitRef`)) (`self.MaxNbOfActionsRequire`)))))
  (if (<= (`local.CurrentStepsNb`) (`local.MaxSteps`))
    (set `local.NormalizedScore` (`KismetMathLibrary.FMax` (`self.MinScore`) (* (/ (`KismetMathLibrary.Conv_IntToDouble` (`local.CurrentStepsNb`)) (`KismetMathLibrary.Conv_IntToDouble` (`local.MaxSteps`))) (`self.MaxScore`))))
    (else
      (set `local.NormalizedScore` (`self.MinScore`))))
  (return (`local.NormalizedScore`)))
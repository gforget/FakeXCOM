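; AI node consideration that scores a candidate tile by whether the unit could see enemies from it in the turn-based tactical game.
; It counts enemies in sight from the target node for the owning unit and checks whether any exist against the WantToHaveEnemyInSight flag.
; A match returns MaxScore and a mismatch returns zero, so the same asset can favor either exposed or hidden positions.
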(fn `ScoreConsiderationNode`
  (params (OwningUnit :type "Unit Object Reference") (TBTacticalGameMode :type "TBTacticalGameMode Object Reference") (TargetNode :type "NodePath Object Reference"))
  (returns (ReturnValue :type "Float (single-precision)"))
  (locals (OwningUnitRef :type "Unit Object Reference") (TBTacticalGameModeRef :type "TBTacticalGameMode Object Reference") (TargetNodeRef :type "NodePath Object Reference") (NormalizedScore :type "Float (double-precision)"))
  (set `local.OwningUnitRef` OwningUnit)
  (set `local.TBTacticalGameModeRef` TBTacticalGameMode)
  (set `local.TargetNodeRef` TargetNode)
  (bind _returnvalue (`self.GetNumberOfEnemyInSight` (`local.OwningUnitRef`) (`local.TBTacticalGameModeRef`) (`local.TargetNodeRef`)))
  (if (== (> _returnvalue 0) (`self.WantToHaveEnemyInSight`))
    (set `local.NormalizedScore` (`self.MaxScore`))
    (else
      (set `local.NormalizedScore` 0.0)))
  (return (`local.NormalizedScore`)))
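; Utility AI action consideration that scores an action by the owning unit's chance to hit the target actor.
; It resolves the action's ability and the target index stored under the preceding action index, then reads that target's hit chance from the unit's ability info.
; The normalized chance, inverted when HighestHitChance is off, is scaled by MaxScore and floored at MinScore.
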(fn `ScoreConsideration`
  (params (OwningUnit :type "Unit Object Reference") (ActionIndex :type Integer) (TBTacticalGameMode :type "TBTacticalGameMode Object Reference"))
  (returns (ReturnValue :type "Float (single-precision)"))
  (locals (OwningUnitRef :type "Unit Object Reference") (TBTacticalGameModeRef :type "TBTacticalGameMode Object Reference") (TargetHitPercentage :type "Float (double-precision)") (AbilityRef :type "UnitAbility Object Reference") (TargetIndexRef :type Integer) (NormalizedScore :type "Float (double-precision)"))
  (bind _value (`BlueprintMapLibrary.Map_Find` (`Unit.UnitAbilityInfos` (`local.OwningUnitRef`)) (`UnitAbility.AbilityId` (`local.AbilityRef`))))
  (set `local.OwningUnitRef` OwningUnit)
  (set `local.TBTacticalGameModeRef` TBTacticalGameMode)
  (set `local.AbilityRef` (`BlueprintMapLibrary.Map_Find` (`Unit.OwnedAbilities` (`local.OwningUnitRef`)) (`AIBrainComponent.GetAbilityIdFromAction` (`Unit.AIBrainComponent` (`local.OwningUnitRef`)) (`self.ActionIndex`))))
  (set `local.TargetIndexRef` (`BlueprintMapLibrary.Map_Find` (`AIBrainComponent.TargetActorIndex` (`Unit.AIBrainComponent` (`local.OwningUnitRef`))) (- (`self.ActionIndex`) 1)))
  (set `local.TargetHitPercentage` (/ (`BlueprintMapLibrary.Map_Find` (`.TargetUnitsHitChances` (break `UnitAbilityInfoStruct` _value)) (`Unit.IdUnit` (`|GetArrayItem` (`.AllAvailableUnitTargets` (break `UnitAbilityInfoStruct` _value)) (`local.TargetIndexRef`)))) 100.0))
  (if (`self.HighestHitChance`)
    (set `local.NormalizedScore` (`local.TargetHitPercentage`))
    (else
      (set `local.NormalizedScore` (- 1.0 (`local.TargetHitPercentage`)))))
  (return (`KismetMathLibrary.FMax` (* (`local.NormalizedScore`) (`self.MaxScore`)) (`self.MinScore`))))
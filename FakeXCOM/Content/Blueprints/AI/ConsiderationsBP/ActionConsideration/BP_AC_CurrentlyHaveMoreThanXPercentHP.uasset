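; An AI action consideration that scores an action by the owning unit's current health percentage.
; It reads two gameplay attributes from the unit's Ability System Component and divides them to get that percentage.
; It returns the max score when the result of comparing against the target percent matches the HaveMoreThanPercentHP flag, otherwise the min score, so one asset covers both above and at-or-below checks.
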(fn `ScoreConsideration`
  (params (OwningUnit :type "Unit Object Reference") (ActionIndex :type Integer) (TBTacticalGameMode :type "TBTacticalGameMode Object Reference"))
  (returns (ReturnValue :type "Float (single-precision)"))
  (locals (OwningUnitRef :type "Unit Object Reference") (UnitHealthPercentage :type "Float (double-precision)") (NormalizedScore :type "Float (double-precision)"))
  (set `local.OwningUnitRef` OwningUnit)
  (set `local.UnitHealthPercentage` (* (/ (`.ReturnValue` (`AbilitySystemComponent.GetGameplayAttributeValue` (`AbilitySystemBlueprintLibrary.GetAbilitySystemComponent` (`local.OwningUnitRef`)) (struct :`AttributeName` "Health" :`Attribute` "/Script/FakeXCOM.UnitAttributeSet:Health" :`AttributeOwner` "/Script/CoreUObject.Class'/Script/FakeXCOM.UnitAttributeSet'"))) (`.ReturnValue` (`AbilitySystemComponent.GetGameplayAttributeValue` (`AbilitySystemBlueprintLibrary.GetAbilitySystemComponent` (`local.OwningUnitRef`)) (struct :`AttributeName` "MaxHealth" :`Attribute` "/Script/FakeXCOM.UnitAttributeSet:MaxHealth" :`AttributeOwner` "/Script/CoreUObject.Class'/Script/FakeXCOM.UnitAttributeSet'")))) 100.0))
  (if (== (> (`local.UnitHealthPercentage`) (`self.TargetPercentHP`)) (`self.HaveMoreThanPercentHP`))
    (set `local.NormalizedScore` (`self.MaxScore`))
    (else
      (set `local.NormalizedScore` (`self.MinScore`))))
  (return (`local.NormalizedScore`)))
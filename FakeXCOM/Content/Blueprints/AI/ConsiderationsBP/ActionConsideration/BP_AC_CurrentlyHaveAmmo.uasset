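; An AI action consideration that scores an action by whether the owning unit's gun currently has ammo.
; ScoreConsideration reads a gameplay attribute from the gun's Ability System Component and treats a value above zero as having ammo.
; It returns TrueScore when that state matches the HaveAmmo setting and FalseScore otherwise, so the same asset can favor either armed or empty states.
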(fn `ScoreConsideration`
  (params (OwningUnit :type "Unit Object Reference") (ActionIndex :type Integer) (TBTacticalGameMode :type "TBTacticalGameMode Object Reference"))
  (returns (ReturnValue :type "Float (single-precision)"))
  (locals (OwningUnitRef :type "Unit Object Reference") (CurrentAmmoAmount :type "Float (double-precision)") (NormalizedScore :type "Float (double-precision)"))
  (set `local.OwningUnitRef` OwningUnit)
  (set `local.CurrentAmmoAmount` (`.ReturnValue` (`AbilitySystemComponent.GetGameplayAttributeValue` (`AbilitySystemBlueprintLibrary.GetAbilitySystemComponent` (`Unit.Gun` (`local.OwningUnitRef`))) (struct :`AttributeName` "Ammo" :`Attribute` "/Script/FakeXCOM.GunAttributeSet:Ammo" :`AttributeOwner` "/Script/CoreUObject.Class'/Script/FakeXCOM.GunAttributeSet'"))))
  (if (== (> (`local.CurrentAmmoAmount`) 0.0) (`self.HaveAmmo`))
    (set `local.NormalizedScore` (`self.TrueScore`))
    (else
      (set `local.NormalizedScore` (`self.FalseScore`))))
  (return (`local.NormalizedScore`)))
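; BP_AC_CurrentPercentHP is an AI action consideration that scores an action by the owning unit's current health percentage in a turn-based tactical game.
; ScoreConsideration divides two attribute values read from the unit's Ability System Component to get that percentage.
; HighHealthPriority selects whether high or low health scores higher, then the result is scaled by MaxScore and floored at MinScore.
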(fn `ScoreConsideration`
  (params (OwningUnit :type "Unit Object Reference") (ActionIndex :type Integer) (TBTacticalGameMode :type "TBTacticalGameMode Object Reference"))
  (returns (ReturnValue :type "Float (single-precision)"))
  (locals (OwningUnitRef :type "Unit Object Reference") (TargetHealthPercentage :type "Float (double-precision)") (NormalizedScore :type "Float (double-precision)"))
  (set `local.OwningUnitRef` OwningUnit)
  (set `local.TargetHealthPercentage` (/ (`.ReturnValue` (`AbilitySystemComponent.GetGameplayAttributeValue` (`AbilitySystemBlueprintLibrary.GetAbilitySystemComponent` (`local.OwningUnitRef`)) (struct :`AttributeName` "Health" :`Attribute` "/Script/FakeXCOM.UnitAttributeSet:Health" :`AttributeOwner` "/Script/CoreUObject.Class'/Script/FakeXCOM.UnitAttributeSet'"))) (`.ReturnValue` (`AbilitySystemComponent.GetGameplayAttributeValue` (`AbilitySystemBlueprintLibrary.GetAbilitySystemComponent` (`local.OwningUnitRef`)) (struct :`AttributeName` "MaxHealth" :`Attribute` "/Script/FakeXCOM.UnitAttributeSet:MaxHealth" :`AttributeOwner` "/Script/CoreUObject.Class'/Script/FakeXCOM.UnitAttributeSet'")))))
  (if (`self.HighHealthPriority`)
    (set `local.NormalizedScore` (`local.TargetHealthPercentage`))
    (else
      (set `local.NormalizedScore` (- 1.0 (`local.TargetHealthPercentage`)))))
  (return (`KismetMathLibrary.FMax` (* (`local.NormalizedScore`) (`self.MaxScore`)) (`self.MinScore`))))
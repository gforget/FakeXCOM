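; AI action consideration that scores an action by the current unit's hit chance with its default ability.
; It looks up that ability's info on the owning unit and reads the hit chance for the first available target, with no comparison across other targets.
; The percentage becomes a fraction scaled by MaxScore, and the score is zero when no targets are available.
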(fn `ScoreConsideration`
  (params (OwningUnit :type "Unit Object Reference") (ActionIndex :type Integer) (TBTacticalGameMode :type "TBTacticalGameMode Object Reference"))
  (returns (ReturnValue :type "Float (single-precision)"))
  (locals (OwningUnitRef :type "Unit Object Reference") (TBTacticalGameModeRef :type "TBTacticalGameMode Object Reference") (DefaultAbilityRef :type "UnitAbility Object Reference") (HitPercentage :type "Float (double-precision)"))
  (bind _owningunitref (`local.OwningUnitRef`))
  (bind _value (`BlueprintMapLibrary.Map_Find` (`Unit.UnitAbilityInfos` (`local.OwningUnitRef`)) (`UnitAbility.AbilityId` (`local.DefaultAbilityRef`))))
  (set `local.OwningUnitRef` OwningUnit)
  (set `local.TBTacticalGameModeRef` TBTacticalGameMode)
  (set `local.DefaultAbilityRef` (`BlueprintMapLibrary.Map_Find` (`Unit.OwnedAbilities` _owningunitref) (`Unit.DefaultAbilityId` _owningunitref)))
  (if (== (`KismetArrayLibrary.Array_Length` (`.AllAvailableUnitTargets` (break `UnitAbilityInfoStruct` (`BlueprintMapLibrary.Map_Find` (`Unit.UnitAbilityInfos` (`local.OwningUnitRef`)) (`UnitAbility.AbilityId` (`local.DefaultAbilityRef`)))))) 0)
    (return 0.0)
    (else
      (set `local.HitPercentage` (/ (`BlueprintMapLibrary.Map_Find` (`.TargetUnitsHitChances` (break `UnitAbilityInfoStruct` _value)) (`Unit.IdUnit` (`|GetArrayItem` (`.AllAvailableUnitTargets` (break `UnitAbilityInfoStruct` _value))))) 100.0))
      (return (* (`local.HitPercentage`) (`self.MaxScore`))))))
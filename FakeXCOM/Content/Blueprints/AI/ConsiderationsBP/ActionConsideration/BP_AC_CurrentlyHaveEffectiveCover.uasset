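; AI action consideration that scores an action on whether the acting unit currently has effective cover in tactical combat.
; It gets the lowest potential defence at the unit's current tile node and treats any value above zero as effective cover.
; The result is compared to the HaveEffectiveCover flag, so the same check can score either having or lacking cover, returning TrueScore on a match and FalseScore otherwise.
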(fn `ScoreConsideration`
  (params (OwningUnit :type "Unit Object Reference") (ActionIndex :type Integer) (TBTacticalGameMode :type "TBTacticalGameMode Object Reference"))
  (returns (ReturnValue :type "Float (single-precision)"))
  (locals (TBTacticalGameModeRef :type "TBTacticalGameMode Object Reference") (OwningUnitRef :type "Unit Object Reference") (OtherUnitRef :type "Unit Object Reference") (NormalizedScore :type "Float (double-precision)") (CoverDefenceScore :type "Float (double-precision)") (OtherDefaultAbilityRef :type "UnitAbility Object Reference") (OtherRangeRef :type "Float (double-precision)") (IsFlanked :type Boolean))
  (set `local.OwningUnitRef` OwningUnit)
  (set `local.TBTacticalGameModeRef` TBTacticalGameMode)
  (bind _returnvalue (`self.GetLowestPotentialDefence` (`local.OwningUnitRef`) (`local.TBTacticalGameModeRef`) (`TileMovementComponent.LocatedNodePath` (`Unit.TileMovementComponent` (`local.OwningUnitRef`)))))
  (set `local.CoverDefenceScore` _returnvalue)
  (if (== (> (`local.CoverDefenceScore`) 0.0) (`self.HaveEffectiveCover`))
    (set `local.NormalizedScore` (`self.TrueScore`))
    (else
      (set `local.NormalizedScore` (`self.FalseScore`))))
  (return (`local.NormalizedScore`)))
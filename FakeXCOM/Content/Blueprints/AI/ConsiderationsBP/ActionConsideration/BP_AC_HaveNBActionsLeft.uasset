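; AI action consideration for a turn-based tactical game that scores an action by the owning unit's action count.
; ScoreConsideration tests whether GetActions exactly equals NbOfActionsToCheck, then compares that result to the HaveActionsLeft flag, which can invert the condition.
; A match returns TrueScore as the normalized score, otherwise FalseScore.
; The action index and game mode inputs are unused.
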(fn `ScoreConsideration`
  (params (OwningUnit :type "Unit Object Reference") (ActionIndex :type Integer) (TBTacticalGameMode :type "TBTacticalGameMode Object Reference"))
  (returns (ReturnValue :type "Float (single-precision)"))
  (locals (NormalizedScore :type "Float (double-precision)"))
  (if (== (== (`Unit.GetActions` OwningUnit) (`self.NbOfActionsToCheck`)) (`self.HaveActionsLeft`))
    (set `local.NormalizedScore` (`self.TrueScore`))
    (else
      (set `local.NormalizedScore` (`self.FalseScore`))))
  (return (`local.NormalizedScore`)))
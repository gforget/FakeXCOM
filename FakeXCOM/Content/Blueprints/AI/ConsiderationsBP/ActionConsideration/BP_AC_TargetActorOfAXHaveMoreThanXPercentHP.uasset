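; AI action consideration that scores an action by whether a target unit's health percentage is above or below a threshold.
; It resolves the action's ability from the AI brain, then picks the target from that ability's available units using the target index stored for the preceding action index.
; A boolean flips the comparison direction, and the result selects one of two configurable scores.
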(fn `ScoreConsideration`
  (params (OwningUnit :type "Unit Object Reference") (ActionIndex :type Integer) (TBTacticalGameMode :type "TBTacticalGameMode Object Reference"))
  (returns (ReturnValue :type "Float (single-precision)"))
  (locals (OwningUnitRef :type "Unit Object Reference") (TargetUnitRef :type "Unit Object Reference") (TBTacticalGameModeRef :type "TBTacticalGameMode Object Reference") (TargetHPPercentage :type "Float (double-precision)") (AbilityRef :type "UnitAbility Object Reference") (TargetActorIndexRef :type Integer) (NormalizedScore :type "Float (double-precision)"))
  (set `local.OwningUnitRef` OwningUnit)
  (set `local.TBTacticalGameModeRef` TBTacticalGameMode)
  (set `local.AbilityRef` (`BlueprintMapLibrary.Map_Find` (`Unit.OwnedAbilities` (`local.OwningUnitRef`)) (`AIBrainComponent.GetAbilityIdFromAction` (`Unit.AIBrainComponent` (`local.OwningUnitRef`)) (`self.ActionIndex`))))
  (set `local.TargetActorIndexRef` (`BlueprintMapLibrary.Map_Find` (`AIBrainComponent.TargetActorIndex` (`Unit.AIBrainComponent` (`local.OwningUnitRef`))) (- (`self.ActionIndex`) 1)))
  (set `local.TargetUnitRef` (`|GetArrayItem` (`.AllAvailableUnitTargets` (break `UnitAbilityInfoStruct` (`BlueprintMapLibrary.Map_Find` (`Unit.UnitAbilityInfos` (`local.OwningUnitRef`)) (`UnitAbility.AbilityId` (`local.AbilityRef`))))) (`local.TargetActorIndexRef`)))
  (set `local.TargetHPPercentage` (/ (`Unit.GetHealth` (`local.TargetUnitRef`)) (`Unit.GetMaxHealth` (`local.TargetUnitRef`))))
  (if (== (> (`local.TargetHPPercentage`) (`self.TargetPercentHP`)) (`self.MoreThanHPPercent`))
    (set `local.NormalizedScore` (`self.TrueScore`))
    (else
      (set `local.NormalizedScore` (`self.FalseScore`))))
  (return (`local.NormalizedScore`)))
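; Action consideration for turn-based tactical AI that scores on whether the owning unit currently has a specific number of actions left.
; ScoreConsideration reads a gameplay attribute from the unit's Ability System Component and tests it for exact equality with NbOfActionsToCheck.
; The HaveActionsLeft flag sets whether a match or a mismatch passes, giving a binary result of MaxScore or MinScore.
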(fn `ScoreConsideration`
  (params (OwningUnit :type "Unit Object Reference") (TBTacticalGameMode :type "TBTacticalGameMode Object Reference"))
  (returns (ReturnValue :type "Float (single-precision)"))
  (locals (NormalizedScore :type "Float (double-precision)"))
  (if (== (== (`.ReturnValue` (`AbilitySystemComponent.GetGameplayAttributeValue` (`AbilitySystemBlueprintLibrary.GetAbilitySystemComponent` OwningUnit) (struct :`AttributeName` "Actions" :`Attribute` "/Script/FakeXCOM.UnitAttributeSet:Actions" :`AttributeOwner` "/Script/CoreUObject.Class'/Script/FakeXCOM.UnitAttributeSet'"))) (`self.NbOfActionsToCheck`)) (`self.HaveActionsLeft`))
    (set `local.NormalizedScore` (`self.MaxScore`))
    (else
      (set `local.NormalizedScore` (`self.MinScore`))))
  (return (`local.NormalizedScore`)))
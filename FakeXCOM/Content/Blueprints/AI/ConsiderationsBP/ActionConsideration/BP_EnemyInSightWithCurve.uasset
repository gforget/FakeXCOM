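; Utility AI action consideration that scores a unit's action by how many enemies are within reach of its default ability.
; It counts the available targets recorded for the unit in its first default ability.
; That count is divided by a highest-enemies-in-sight value and fed into a runtime float curve, whose output is the score.
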(fn `ScoreConsideration`
  (params (OwningUnit :type "Unit Object Reference") (TBTacticalGameMode :type "TBTacticalGameMode Object Reference"))
  (returns (ReturnValue :type "Float (single-precision)"))
  (locals (UnitRef :type "Unit Object Reference") (DefaultAbilityRef :type "UnitAbility Object Reference") (CurrentNumberOfTarget :type Integer :default 0))
  (set `local.UnitRef` OwningUnit)
  (set `local.DefaultAbilityRef` (`|GetArrayItem` (`Unit.OwnedAbilities` (`local.UnitRef`)) (`|GetArrayItem` (`Unit.DefaultAbilitiesIndexes` (`local.UnitRef`)))))
  (set `local.CurrentNumberOfTarget` (`KismetArrayLibrary.Array_Length` (`.AllAvailableTargets` (break `UnitAbilityInfoStruct` (`BlueprintMapLibrary.Map_Find` (`UnitAbility.UnitAbilityInfos` (`local.DefaultAbilityRef`)) (`Unit.IdUnit` (`local.UnitRef`)))))))
  (return (`MyFunctionLibrary.GetRuntimeFloatCurveValue` (`self.Curve`) (/ (`KismetMathLibrary.Conv_IntToDouble` (`local.CurrentNumberOfTarget`)) (`KismetMathLibrary.Conv_IntToDouble` (`self.HighestNBEnemiesInSight`))))))
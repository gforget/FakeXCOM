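; BP_AC_CanUseUnitAbility is an AI action consideration that scores an action by whether the owning unit can use a given ability.
; ScoreConsideration checks the configured AbilityID on the unit through CheckAbilityById and compares the result with CanUseUnitAbility.
; It returns TrueScore on a match and FalseScore otherwise as the normalized score, ignoring the action index and game mode.
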(fn `ScoreConsideration`
  (params (OwningUnit :type "Unit Object Reference") (ActionIndex :type Integer) (TBTacticalGameMode :type "TBTacticalGameMode Object Reference"))
  (returns (ReturnValue :type "Float (single-precision)"))
  (locals (OwningUnitRef :type "Unit Object Reference") (NormalizedScore :type "Float (double-precision)"))
  (set `local.OwningUnitRef` OwningUnit)
  (bind _returnvalue (`Unit.CheckAbilityById` (`local.OwningUnitRef`) (`self.AbilityID`)))
  (if (== _returnvalue (`self.CanUseUnitAbility`))
    (set `local.NormalizedScore` (`self.TrueScore`))
    (else
      (set `local.NormalizedScore` (`self.FalseScore`))))
  (return (`local.NormalizedScore`)))
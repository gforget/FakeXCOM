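; Utility AI action consideration that scores a unit's action by whether it has a target actor assigned.
; It looks up the action index in the AI brain component's target actor index map and treats -1 as no target.
; The score is MaxScore when that result matches the HaveATargetActor flag, otherwise MinScore, so the same check can favor having or lacking a target.
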(fn `ScoreConsideration`
  (params (OwningUnit :type "Unit Object Reference") (ActionIndex :type Integer) (TBTacticalGameMode :type "TBTacticalGameMode Object Reference"))
  (returns (ReturnValue :type "Float (single-precision)"))
  (locals (UnitRef :type "Unit Object Reference") (ActionIndexRef :type Integer) (NormalizedScore :type "Float (double-precision)"))
  (set `local.UnitRef` OwningUnit)
  (set `local.ActionIndexRef` ActionIndex)
  (if (== (!= (`BlueprintMapLibrary.Map_Find` (`AIBrainComponent.TargetActorIndex` (`Unit.AIBrainComponent` (`local.UnitRef`))) (`local.ActionIndexRef`)) -1) (`self.HaveATargetActor`))
    (set `local.NormalizedScore` (`self.MaxScore`))
    (else
      (set `local.NormalizedScore` (`self.MinScore`))))
  (return (`local.NormalizedScore`)))
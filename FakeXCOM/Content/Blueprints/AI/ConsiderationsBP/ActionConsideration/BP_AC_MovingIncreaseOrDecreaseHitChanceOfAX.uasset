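; AI action consideration that scores a move by whether its target node improves the unit's default ability hit chance.
; It finds the best hit chance from that node among faction-valid targets passing death and line-of-sight checks.
; It compares this with the cached chance on the previous action index's target, or zero without one.
; HaveBetterHitChance selects whether improvement or its absence returns TrueScore; otherwise it returns FalseScore.
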(fn `ScoreConsideration`
  (params (OwningUnit :type "Unit Object Reference") (ActionIndex :type Integer) (TBTacticalGameMode :type "TBTacticalGameMode Object Reference"))
  (returns (ReturnValue :type "Float (single-precision)"))
  (locals (OwningUnitRef :type "Unit Object Reference") (SelfActionIndexRef :type Integer :default 0) (TBTacticalGameModeRef :type "TBTacticalGameMode Object Reference") (DefaultAbilityRef :type "UnitAbility Object Reference") (PotentialTargetRef :type "Unit Object Reference") (TargetNodeHitChance :type "Float (double-precision)") (BestCurrentHitChance :type "Float (double-precision)") (NormalizedScore :type "Float (double-precision)") (TargetIndexRef :type Integer))
  (bind _owningunitref (`local.OwningUnitRef`))
  (bind _value (`BlueprintMapLibrary.Map_Find` (`Unit.UnitAbilityInfos` (`local.OwningUnitRef`)) (`UnitAbility.AbilityId` (`local.DefaultAbilityRef`))))
  (set `local.OwningUnitRef` OwningUnit)
  (set `local.SelfActionIndexRef` ActionIndex)
  (set `local.TBTacticalGameModeRef` TBTacticalGameMode)
  (set `local.DefaultAbilityRef` (`BlueprintMapLibrary.Map_Find` (`Unit.OwnedAbilities` _owningunitref) (`Unit.DefaultAbilityId` _owningunitref)))
  (set `local.TargetNodeHitChance` 0.0)
  (for _array_element (`TargetManager.GetAllValidUnitIdFromFactionRelation` (`TBTacticalGameMode.TargetManager` (`local.TBTacticalGameModeRef`)) (`local.OwningUnitRef`) (`UnitAbility.ValidTargetFactionRelation` (`local.DefaultAbilityRef`)))
    (bind _returnvalue (`UnitManager.GetUnitFromId` (`TBTacticalGameMode.UnitManager` (`local.TBTacticalGameModeRef`)) _array_element))
    (bind _output_get (set `local.PotentialTargetRef` _returnvalue))
    (bind _returnvalue_2 (`TargetManager.ValidateTargetDeathFilter` (`TBTacticalGameMode.TargetManager` (`local.TBTacticalGameModeRef`)) _output_get (`UnitAbility.DeadTargetFilter` (`local.DefaultAbilityRef`))))
    (if _returnvalue_2
      (bind _returnvalue_3 (`TargetManager.ConfirmLineOfSightOnUnit` (`TBTacticalGameMode.TargetManager` (`local.TBTacticalGameModeRef`)) (`local.OwningUnitRef`) (`local.PotentialTargetRef`) (+ (`SceneComponent.K2_GetComponentLocation` (`BlueprintMapLibrary.Map_Find` (`AIBrainComponent.TargetNodePath` (`Unit.AIBrainComponent` (`local.OwningUnitRef`))) (`local.SelfActionIndexRef`))) (`KismetMathLibrary.MakeVector` 0.0 0.0 (`Unit.ZGroundOffset` (`local.OwningUnitRef`)))) (`Actor.K2_GetActorLocation` (`local.PotentialTargetRef`)) (`UnitAbility.GetRangeValue` (`local.DefaultAbilityRef`) (`local.OwningUnitRef`))))
      (if _returnvalue_3
        (bind _returnvalue_4 (`UnitAbility.GetHitChance` (`local.DefaultAbilityRef`) (`local.OwningUnitRef`) (`local.PotentialTargetRef`) (`BlueprintMapLibrary.Map_Find` (`AIBrainComponent.TargetNodePath` (`Unit.AIBrainComponent` (`local.OwningUnitRef`))) (`local.SelfActionIndexRef`)) (`TileMovementComponent.LocatedNodePath` (`Unit.TileMovementComponent` (`local.PotentialTargetRef`)))))
        (if (> _returnvalue_4 (`local.TargetNodeHitChance`))
          (set `local.TargetNodeHitChance` _returnvalue_4)))))
  (set `local.TargetIndexRef` (`BlueprintMapLibrary.Map_Find` (`AIBrainComponent.TargetActorIndex` (`Unit.AIBrainComponent` (`local.OwningUnitRef`))) (- (`self.ActionIndex`) 1)))
  (if (!= (`local.TargetIndexRef`) -1)
    (set `local.BestCurrentHitChance` (/ (`BlueprintMapLibrary.Map_Find` (`.TargetUnitsHitChances` (break `UnitAbilityInfoStruct` _value)) (`Unit.IdUnit` (`|GetArrayItem` (`.AllAvailableUnitTargets` (break `UnitAbilityInfoStruct` _value)) (`local.TargetIndexRef`)))) 100.0))
    (else
      (set `local.BestCurrentHitChance` 0.0)))
  (if (== (> (`local.TargetNodeHitChance`) (`local.BestCurrentHitChance`)) (`self.HaveBetterHitChance`))
    (set `local.NormalizedScore` (`self.TrueScore`))
    (else
      (set `local.NormalizedScore` (`self.FalseScore`))))
  (return (`local.NormalizedScore`)))
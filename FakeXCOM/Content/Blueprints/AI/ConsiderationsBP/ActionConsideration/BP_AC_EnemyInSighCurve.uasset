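; AI action consideration that scores an action by how many enemies the unit can currently target.
; It looks up the unit's default ability and counts that unit's available targets in the ability's info map.
; That count, divided by the highest enemies-in-sight number, is sampled on a runtime float curve to produce the score.
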(fn `ScoreConsideration`
  (params (OwningUnit :type "Unit Object Reference") (ActionIndex :type Integer) (TBTacticalGameMode :type "TBTacticalGameMode Object Reference"))
  (returns (ReturnValue :type "Float (single-precision)"))
  (locals (UnitRef :type "Unit Object Reference") (DefaultAbilityRef :type "UnitAbility Object Reference") (CurrentNumberOfTarget :type Integer :default 0))
  (bind _unitref (`local.UnitRef`))
  (set `local.UnitRef` OwningUnit)
  (set `local.DefaultAbilityRef` (`BlueprintMapLibrary.Map_Find` (`Unit.OwnedAbilities` _unitref) (`Unit.DefaultAbilityId` _unitref)))
  (set `local.CurrentNumberOfTarget` (`KismetArrayLibrary.Array_Length` (`.AllAvailableTargets` (break `UnitAbilityInfoStruct` (`BlueprintMapLibrary.Map_Find` (`UnitAbility.UnitAbilityInfos` (`local.DefaultAbilityRef`)) (`Unit.IdUnit` (`local.UnitRef`)))))))
  (return (`MyFunctionLibrary.GetRuntimeFloatCurveValue` (`self.Curve`) (/ (`KismetMathLibrary.Conv_IntToDouble` (`local.CurrentNumberOfTarget`)) (`KismetMathLibrary.Conv_IntToDouble` (`self.HighestNBEnemiesInSight`))))))
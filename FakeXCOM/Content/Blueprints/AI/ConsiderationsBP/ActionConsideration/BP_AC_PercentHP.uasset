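; Action consideration for tactical AI that scores an action by the acting unit's current health percentage.
; ScoreConsideration divides the owning unit's health by its max health, inverting the ratio unless HighHealthPriority is set.
; The result is scaled by MaxScore and floored at MinScore.
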(fn `ScoreConsideration`
  (params (OwningUnit :type "Unit Object Reference") (ActionIndex :type Integer) (TBTacticalGameMode :type "TBTacticalGameMode Object Reference"))
  (returns (ReturnValue :type "Float (single-precision)"))
  (locals (OwningUnitRef :type "Unit Object Reference") (TargetHealthPercentage :type "Float (double-precision)") (NormalizedScore :type "Float (double-precision)"))
  (set `local.OwningUnitRef` OwningUnit)
  (set `local.TargetHealthPercentage` (/ (`Unit.GetHealth` (`local.OwningUnitRef`)) (`Unit.GetMaxHealth` (`local.OwningUnitRef`))))
  (if (`self.HighHealthPriority`)
    (set `local.NormalizedScore` (`local.TargetHealthPercentage`))
    (else
      (set `local.NormalizedScore` (- 1.0 (`local.TargetHealthPercentage`)))))
  (return (`KismetMathLibrary.FMax` (* (`local.NormalizedScore`) (`self.MaxScore`)) (`self.MinScore`))))
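; AI action consideration that scores an action by whether any movement node gives the unit an enemy in sight.
; It gathers the unit's base-distance and long-distance nodes from its AI brain component and checks each for visible enemy units, stopping at the first hit.
; It returns the true score when the result matches the configured HavePotentialTarget flag, otherwise the false score, so the same check can favor either outcome.
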(fn `ScoreConsideration`
  (params (OwningUnit :type "Unit Object Reference") (ActionIndex :type Integer) (TBTacticalGameMode :type "TBTacticalGameMode Object Reference"))
  (returns (ReturnValue :type "Float (single-precision)"))
  (locals (TBTacticalGameModeRef :type "TBTacticalGameMode Object Reference") (OwningUnitRef :type "Unit Object Reference") (AllNodesPath :type "Array of NodePath Object Reference") (FoundTarget :type Boolean) (NormalizedScore :type "Float (double-precision)"))
  (set `local.OwningUnitRef` OwningUnit)
  (set `local.TBTacticalGameModeRef` TBTacticalGameMode)
  (set `local.FoundTarget` false)
  (`KismetArrayLibrary.Array_Append` (`local.AllNodesPath`) (`AIBrainComponent.AllBaseDistanceNode` (`Unit.AIBrainComponent` (`local.OwningUnitRef`))))
  (`KismetArrayLibrary.Array_Append` (`local.AllNodesPath`) (`AIBrainComponent.AllLongDistanceNode` (`Unit.AIBrainComponent` (`local.OwningUnitRef`))))
  (for _array_element (`local.AllNodesPath`)
    (bind _returnvalue (`self.GetAllEnemyUnitInSight` (`local.OwningUnitRef`) (`local.TBTacticalGameModeRef`) _array_element))
    (if (> (`KismetArrayLibrary.Array_Length` _returnvalue) 0)
      (set `local.FoundTarget` true)
      (break)))
  (if (== (`self.HavePotentialTarget`) (`local.FoundTarget`))
    (set `local.NormalizedScore` (`self.TrueScore`))
    (else
      (set `local.NormalizedScore` (`self.FalseScore`))))
  (return (`local.NormalizedScore`)))
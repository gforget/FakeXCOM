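; BP_AC_HaveAmmo is an AI action consideration for the tactical game that scores an action on whether the owning unit's gun has ammo.
; ScoreConsideration reads the gun's ammo count and compares the "above zero" result to the HaveAmmo flag, so one asset can test for either loaded or empty.
; It returns TrueScore on a match and FalseScore otherwise as the normalized score, ignoring the action index and game mode inputs.
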(fn `ScoreConsideration`
  (params (OwningUnit :type "Unit Object Reference") (ActionIndex :type Integer) (TBTacticalGameMode :type "TBTacticalGameMode Object Reference"))
  (returns (ReturnValue :type "Float (single-precision)"))
  (locals (OwningUnitRef :type "Unit Object Reference") (CurrentAmmoAmount :type Integer) (NormalizedScore :type "Float (double-precision)"))
  (set `local.OwningUnitRef` OwningUnit)
  (set `local.CurrentAmmoAmount` (`Gun.GetAmmo` (`Unit.Gun` (`local.OwningUnitRef`))))
  (if (== (> (`local.CurrentAmmoAmount`) 0) (`self.HaveAmmo`))
    (set `local.NormalizedScore` (`self.TrueScore`))
    (else
      (set `local.NormalizedScore` (`self.FalseScore`))))
  (return (`local.NormalizedScore`)))
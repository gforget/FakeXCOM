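; An AI action consideration that scores an action by whether the owning unit's health is above a percentage threshold.
; ScoreConsideration converts current over max health to a percentage and compares it to TargetPercentHP.
; A HaveMoreThanPercentHP flag can invert the test, so the same asset also covers at-or-below checks.
; It returns TrueScore on a match and FalseScore otherwise as the normalized score.
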(fn `ScoreConsideration`
  (params (OwningUnit :type "Unit Object Reference") (ActionIndex :type Integer) (TBTacticalGameMode :type "TBTacticalGameMode Object Reference"))
  (returns (ReturnValue :type "Float (single-precision)"))
  (locals (OwningUnitRef :type "Unit Object Reference") (UnitHealthPercentage :type "Float (double-precision)") (NormalizedScore :type "Float (double-precision)"))
  (set `local.OwningUnitRef` OwningUnit)
  (set `local.UnitHealthPercentage` (* (/ (`Unit.GetHealth` (`local.OwningUnitRef`)) (`Unit.GetMaxHealth` (`local.OwningUnitRef`))) 100.0))
  (if (== (> (`local.UnitHealthPercentage`) (`self.TargetPercentHP`)) (`self.HaveMoreThanPercentHP`))
    (set `local.NormalizedScore` (`self.TrueScore`))
    (else
      (set `local.NormalizedScore` (`self.FalseScore`))))
  (return (`local.NormalizedScore`)))
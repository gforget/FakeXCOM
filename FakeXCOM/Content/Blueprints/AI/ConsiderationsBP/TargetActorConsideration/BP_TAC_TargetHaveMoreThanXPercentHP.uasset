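; A target actor consideration for tactical AI action scoring that rates a target unit by whether its health is above a set percentage.
; It casts the target to Unit, converts current over max health to a percentage and compares that with TargetPercentHP.
; The HaveMoreThanPercentHP flag can invert the test, and the result selects TrueScore or FalseScore as the normalized score.
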(fn `ScoreConsiderationActor`
  (params (OwningUnit :type "Unit Object Reference") (ActionIndex :type Integer) (TBTacticalGameMode :type "TBTacticalGameMode Object Reference") (TargetActor :type "Actor Object Reference"))
  (returns (ReturnValue :type "Float (single-precision)"))
  (locals (TargetUnitRef :type "Unit Object Reference") (TargetUnitHealthPercentage :type "Float (double-precision)") (NormalizedScore :type "Float (double-precision)"))
  (bind _asunit (cast `Unit` TargetActor))
  (set `local.TargetUnitRef` _asunit)
  (set `local.TargetUnitHealthPercentage` (* (/ (`Unit.GetHealth` (`local.TargetUnitRef`)) (`Unit.GetMaxHealth` (`local.TargetUnitRef`))) 100.0))
  (if (== (> (`local.TargetUnitHealthPercentage`) (`self.TargetPercentHP`)) (`self.HaveMoreThanPercentHP`))
    (set `local.NormalizedScore` (`self.TrueScore`))
    (else
      (set `local.NormalizedScore` (`self.FalseScore`))))
  (return (`local.NormalizedScore`)))
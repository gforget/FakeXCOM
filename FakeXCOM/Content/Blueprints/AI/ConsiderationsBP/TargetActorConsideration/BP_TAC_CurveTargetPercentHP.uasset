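; A utility AI target actor consideration that scores a candidate target by its remaining health percentage.
; It casts the target actor to a Unit and divides its current health by its max health.
; That ratio is the input to a runtime float curve, whose value becomes the score, so the curve shapes how health affects target preference.
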(fn `ScoreConsiderationActor`
  (params (OwningUnit :type "Unit Object Reference") (ActionIndex :type Integer) (TBTacticalGameMode :type "TBTacticalGameMode Object Reference") (TargetActor :type "Actor Object Reference"))
  (returns (ReturnValue :type "Float (single-precision)"))
  (locals (TargetUnitRef :type "Unit Object Reference") (TargetHealthPercentage :type "Float (double-precision)") (NormalizedScore :type "Float (double-precision)"))
  (bind _asunit (cast `Unit` TargetActor))
  (set `local.TargetUnitRef` _asunit)
  (set `local.TargetHealthPercentage` (/ (`Unit.GetHealth` (`local.TargetUnitRef`)) (`Unit.GetMaxHealth` (`local.TargetUnitRef`))))
  (return (`MyFunctionLibrary.GetRuntimeFloatCurveValue` (`self.Curve`) (`local.TargetHealthPercentage`))))
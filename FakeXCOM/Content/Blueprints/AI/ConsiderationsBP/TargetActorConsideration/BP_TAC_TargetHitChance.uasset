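; Utility AI target consideration that scores a candidate target unit by how likely the owning unit is to hit it.
; It looks up the owning unit's default ability and asks it for hit chance using both units' currently located node paths.
; The percentage is normalized and scaled by MaxScore, so the default ability's odds are used regardless of the action index.
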(fn `ScoreConsiderationActor`
  (params (OwningUnit :type "Unit Object Reference") (ActionIndex :type Integer) (TBTacticalGameMode :type "TBTacticalGameMode Object Reference") (TargetActor :type "Actor Object Reference"))
  (returns (ReturnValue :type "Float (single-precision)"))
  (locals (TargetUnitRef :type "Unit Object Reference") (OwningUnitRef :type "Unit Object Reference") (DefaultAbilityRef :type "UnitAbility Object Reference") (NormalizedScore :type "Float (single-precision)" :default 0.0))
  (bind _owningunitref (`local.OwningUnitRef`))
  (set `local.OwningUnitRef` OwningUnit)
  (bind _asunit (cast `Unit` TargetActor))
  (set `local.TargetUnitRef` _asunit)
  (set `local.DefaultAbilityRef` (`BlueprintMapLibrary.Map_Find` (`Unit.OwnedAbilities` _owningunitref) (`Unit.DefaultAbilityId` _owningunitref)))
  (bind _returnvalue (`UnitAbility.GetHitChance` (`local.DefaultAbilityRef`) (`local.OwningUnitRef`) (`local.TargetUnitRef`) (`TileMovementComponent.LocatedNodePath` (`Unit.TileMovementComponent` (`local.OwningUnitRef`))) (`TileMovementComponent.LocatedNodePath` (`Unit.TileMovementComponent` (`local.TargetUnitRef`)))))
  (set `local.NormalizedScore` (/ _returnvalue 100.0))
  (return (* (`local.NormalizedScore`) (`self.MaxScore`))))
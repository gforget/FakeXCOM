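; Target actor consideration for the turn-based tactical AI that scores a candidate target unit by its health percentage.
; It casts the target to Unit and divides two gameplay attribute values read from that unit's Ability System Component to get the health fraction.
; The HighHealthPriority flag selects whether that fraction or its inverse becomes the normalized score, favoring either healthy or wounded targets.
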(fn `ScoreConsiderationActor`
  (params (OwningUnit :type "Unit Object Reference") (TBTacticalGameMode :type "TBTacticalGameMode Object Reference") (TargetActor :type "Actor Object Reference"))
  (returns (ReturnValue :type "Float (single-precision)"))
  (locals (TargetUnitRef :type "Unit Object Reference") (TargetHealthPercentage :type "Float (double-precision)") (NormalizedScore :type "Float (double-precision)"))
  (bind _asunit (cast `Unit` TargetActor))
  (set `local.TargetUnitRef` _asunit)
  (set `local.TargetHealthPercentage` (/ (`.ReturnValue` (`AbilitySystemComponent.GetGameplayAttributeValue` (`AbilitySystemBlueprintLibrary.GetAbilitySystemComponent` (`local.TargetUnitRef`)) (struct :`AttributeName` "Health" :`Attribute` "/Script/FakeXCOM.UnitAttributeSet:Health" :`AttributeOwner` "/Script/CoreUObject.Class'/Script/FakeXCOM.UnitAttributeSet'"))) (`.ReturnValue` (`AbilitySystemComponent.GetGameplayAttributeValue` (`AbilitySystemBlueprintLibrary.GetAbilitySystemComponent` (`local.TargetUnitRef`)) (struct :`AttributeName` "MaxHealth" :`Attribute` "/Script/FakeXCOM.UnitAttributeSet:MaxHealth" :`AttributeOwner` "/Script/CoreUObject.Class'/Script/FakeXCOM.UnitAttributeSet'")))))
  (if (`self.HighHealthPriority`)
    (set `local.NormalizedScore` (`local.TargetHealthPercentage`))
    (else
      (set `local.NormalizedScore` (- 1.0 (`local.TargetHealthPercentage`)))))
  (return (`local.NormalizedScore`)))
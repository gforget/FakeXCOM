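; Gameplay ability for AI units that starts movement along the node path belonging to the chosen action.
; On activation it casts the owning actor to Unit, then looks up the AIBrainComponent's TargetNodePath map by ChosenActionIndex.
; It passes that path to the unit's MoveToNodePath and ends immediately afterward, with no wait for a movement-completion event.
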(event `self.K2_ActivateAbility`
  (bind _aibraincomponent (`Unit.AIBrainComponent` (`self.OwningUnitRef`)))
  (bind _asunit (cast `Unit` (`self.GetOwningActorFromActorInfo`)))
  (set `self.OwningUnitRef` _asunit)
  (`Unit.MoveToNodePath` (`self.OwningUnitRef`) (`BlueprintMapLibrary.Map_Find` (`AIBrainComponent.TargetNodePath` _aibraincomponent) (`AIBrainComponent.ChosenActionIndex` _aibraincomponent)))
  (`self.K2_EndAbility`))
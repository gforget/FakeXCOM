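; BP_ShootTargetActor is an AI unit ability that makes the owning unit shoot the target chosen by its AI brain.
; On activation it looks up the target index for the brain's chosen action and selects that target through the tactical game mode's TargetManager.
; It then triggers the unit's "Shoot" ability by ID and ends itself, printing a debug message if no target is set or activation fails.
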(event `self.K2_ActivateAbility`
  (bind _aibraincomponent (`Unit.AIBrainComponent` (`self.OwningUnitRef`)))
  (bind _aibraincomponent_2 (`Unit.AIBrainComponent` (`self.OwningUnitRef`)))
  (bind _asunit (cast `Unit` (`self.GetOwningActorFromActorInfo`)))
  (set `self.OwningUnitRef` _asunit)
  (if (!= (`BlueprintMapLibrary.Map_Find` (`AIBrainComponent.TargetActorIndex` _aibraincomponent) (`AIBrainComponent.ChosenActionIndex` _aibraincomponent)) -1)
    (`TargetManager.SelectTarget` (`TBTacticalGameMode.TargetManager` (`self.GetTBTacticalGameMode`)) (`BlueprintMapLibrary.Map_Find` (`AIBrainComponent.TargetActorIndex` _aibraincomponent_2) (`AIBrainComponent.ChosenActionIndex` _aibraincomponent_2)))
    (bind _returnvalue (`Unit.TryActivateAbilityByID` (`self.OwningUnitRef`) "Shoot" false))
    (if (not _returnvalue)
      (`KismetSystemLibrary.PrintString` "Unit doesn't have shoot ability"))
    (`self.K2_EndAbility`)
    (else
      (`KismetSystemLibrary.PrintString` "No Target Selected" true true (struct :`R` 1.0 :`G` 0.009844 :`A` 1.0))
      (`self.K2_EndAbility`))))